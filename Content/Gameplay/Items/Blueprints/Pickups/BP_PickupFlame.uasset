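; Flame pickup for a Bomberman-style game that increases the flame length of the player pawn that touches it.
; On overlap it casts the other actor to BP_BombermanPawn, raises its flame length by one and destroys itself.
; Tick counts down an invulnerability timer, then makes the Damageable vulnerable and switches off its own ticking.
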(event EventBeginPlay
  (|CallParentFunction) ; This node is disabled and will not be called.\nDrag off pins to build functionality.
)

(event Collision|EventActorBeginOverlap
  (params (OtherActor :type Actor%20Object%20Reference))
  (|CallParentFunction OtherActor)
  (bind _asbp_bomberman_pawn (Utilities|Casting|CastToBP_BombermanPawn OtherActor))
  (Class|BombermanPawn|IncreaseFlameLength _asbp_bomberman_pawn 1)
  (Actor|DestroyActor))

(event EventTick
  (params (DeltaSeconds :type Float%20%28single-precision%29))
  (|CallParentFunction DeltaSeconds)
  (if (> (Variables|Default|GetInvulnerabilityTimer) 0.0)
    (bind _output_get (Variables|Default|SetInvulnerabilityTimer (- (Variables|Default|GetInvulnerabilityTimer) DeltaSeconds)))
    (if (<= _output_get 0.0)
      (Variables|/Script/BombermanLike.DamageableComponent|SetbInvulnerable (Variables|Default|GetDamageable) false)
      (Actor|Tick|SetActorTickEnabled false))))

(fn ConstructionScript
  (|CallParentFunction))